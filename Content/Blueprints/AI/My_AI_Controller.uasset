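; AI controller that feeds looping waypoint patrol targets to the BT_AI behavior tree through the blackboard.
; BeginPlay matches the nearest SpawnPoint's array index to Waypoint.WaypointIndex to build its route.
; It targets the closest waypoint, calling RunBehaviorTree inside that search loop whenever a nearer one is found.
; Tick writes the pawn's waypoint distance to the blackboard and advances the target when close, wrapping at the end.
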(event `self.ReceiveTick`
  (params (DeltaSeconds :type "Float (single-precision)"))
  (bind _returnvalue (`AIBlueprintHelperLibrary.GetBlackboard` self))
  (bind _returnvalue_2 (+ (`self.WaypointIndex`) 1))
  (bind _aswaypoint (cast `/Game/Blueprints/AI/Waypoint` (`BlackboardComponent.GetValueAsObject` _returnvalue (`self.Waypoints Key`))))
  (bind _returnvalue_3 (`self.GetDistanceTo` _aswaypoint (`self.K2_GetPawn`)))
  (`BlackboardComponent.SetValueAsFloat` _returnvalue (`self.WaypointDistance Key`) _returnvalue_3)
  (if (< _returnvalue_3 150.0)
    (if (> _returnvalue_2 (`KismetArrayLibrary.Array_LastIndex` (`self.Waypoint_Array`)))
      (bind _output_get (set `self.WaypointIndex` 0))
      (`BlackboardComponent.SetValueAsObject` (`AIBlueprintHelperLibrary.GetBlackboard` self) (`self.Waypoints Key`) (`|GetArrayItem` (`self.Waypoint_Array`) _output_get))
      (else
        (bind _output_get_2 (set `self.WaypointIndex` _returnvalue_2))
        (`BlackboardComponent.SetValueAsObject` (`AIBlueprintHelperLibrary.GetBlackboard` self) (`self.Waypoints Key`) (`|GetArrayItem` (`self.Waypoint_Array`) _output_get_2))))))

(event `self.ReceiveBeginPlay`
  (bind _outactors (`GameplayStatics.GetAllActorsOfClass` "/Game/Blueprints/AI/SpawnPoint.SpawnPoint_C"))
  (bind _output_get (set `self.SpawnPoints_Array` _outactors))
  (for (_array_element _array_index) _output_get
    (bind _returnvalue (`self.GetDistanceTo` _array_element self))
    (if (< _returnvalue (`self.SpawnPointDistanceTEMP`))
      (set `self.SpawnPointDistanceTEMP` _returnvalue)
      (set `self.Own_Index` _array_index)))
  (bind _outactors_2 (`GameplayStatics.GetAllActorsOfClass` "/Game/Blueprints/AI/Waypoint.Waypoint_C"))
  (for _array_element_2 _outactors_2
    (if (== (`self.Own_Index`) (`/Game/Blueprints/AI/Waypoint.WaypointIndex` _array_element_2))
      (`KismetArrayLibrary.Array_Add` (`self.Waypoint_Array`) _array_element_2)))
  (for _array_element_3 (`self.Waypoint_Array`)
    (`KismetArrayLibrary.Array_Add` (`self.WaypointDistances`) (`self.GetDistanceTo` _array_element_3)))
  (for (_array_element_4 _array_index_2) (`self.WaypointDistances`)
    (if (< _array_element_4 (`self.DistanceTemp`))
      (set `self.DistanceTemp` _array_element_4)
      (bind _output_get_2 (set `self.WaypointIndex` _array_index_2))
      (`BlackboardComponent.SetValueAsObject` (`AIBlueprintHelperLibrary.GetBlackboard` self) (`self.Waypoints Key`) (`|GetArrayItem` (`self.Waypoint_Array`) _output_get_2))
      (`self.RunBehaviorTree` "/Game/Blueprints/AI/BT_AI.BT_AI"))))

(fn `UserConstructionScript`)