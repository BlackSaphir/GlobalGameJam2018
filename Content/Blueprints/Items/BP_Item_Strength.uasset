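; BP_Item_Strength is a pickup item that boosts the player's strength when touched.
; On BeginPlay it caches the first BP_GamePlayManager in the level and the player's ThirdPersonCharacter.
; When that character overlaps it, it adds its own Strength to the manager's total, calls StartStrengthBuff on the manager, then destroys itself after a short delay.
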(event `self.ReceiveBeginPlay`
  (`|ExecutionSequence`
    (:`then_0`
      (bind _outactors (`GameplayStatics.GetAllActorsOfClass` "/Game/Blueprints/Gameplay/BP_GamePlayManager.BP_GamePlayManager_C"))
      (set `self.GamePlayManagerRef` (`|GetArrayItem` _outactors)))
    (:`then_1`
      (bind _asthird_person_character (cast `/Game/Blueprints/Character/ThirdPersonCharacter` (`GameplayStatics.GetPlayerCharacter` 0)))
      (set `self.Char_Ref` _asthird_person_character))))

(event `self.ReceiveActorBeginOverlap`
  (params (OtherActor :type "Actor Object Reference"))
  (if (== OtherActor (`self.Char_Ref`))
    (set `/Game/Blueprints/Gameplay/BP_GamePlayManager.Strength` (+ (`self.strength`) (`/Game/Blueprints/Gameplay/BP_GamePlayManager.Strength` (`self.GamePlayManagerRef`))) (`self.GamePlayManagerRef`))
    (`/Game/Blueprints/Gameplay/BP_GamePlayManager.Start_Strength_Buff` (`self.GamePlayManagerRef`))
    (`KismetSystemLibrary.Delay` 0.2)
    (`self.K2_DestroyActor`)))

(fn `UserConstructionScript`)